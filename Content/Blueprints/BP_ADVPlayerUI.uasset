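; Player-side Blueprint that drives the HUD and handles talk and pause-menu keys.
; BeginPlay creates UI_Screen and, after a short delay, pushes HP, stamina and magazine values to it; Tick refreshes only stamina and magazine.
; F calls TalkMessage on every overlapping BP_GuildNPC.
; Escape opens PauseMenu with UI-only input and pauses the game, while K opens the same menu with the game unpaused.
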(event EventBeginPlay
  (bind _returnvalue (UserInterface|CreateWidget "/Game/UIs/UI_Screen.UI_Screen_C" (Game|GetPlayerController 0)))
  (Variables|Default|SetuiScreen _returnvalue)
  (UserInterface|Viewport|AddtoViewport (Variables|Default|GetuiScreen) 0)
  (Utilities|FlowControl|Delay 0.05)
  (CallFunction|UiCtrlHP)
  (CallFunction|UiCtrlSP)
  (CallFunction|UiCtrlMagazine))

(event Collision|EventActorBeginOverlap
  (params (OtherActor :type Actor%20Object%20Reference)))

(event EventTick
  (params (DeltaSeconds :type Float%20%28single-precision%29))
  (CallFunction|UiCtrlSP)
  (CallFunction|UiCtrlMagazine))

(event Input|KeyboardEvents|F
  (params (Key :type Key%20Structure :default "None"))
  (:Pressed
    (for _array_element (Collision|GetOverlappingActors "/Game/Blueprints/BP_GuildNPC.BP_GuildNPC_C" :!class /Script/Engine.Actor)
      (if true
        (Class|BPIDialogue|Talk(Message) _array_element)))))

(event Input|KeyboardEvents|K
  (params (Key :type Key%20Structure :default "None"))
  (bind _returnvalue (Game|GetPlayerController 0))
  (:Pressed
    (bind _returnvalue_2 (UserInterface|CreateWidget "/Game/Blueprints/PauseMenu.PauseMenu_C"))
    (UserInterface|Viewport|AddtoViewport _returnvalue_2 0)
    (Game|SetGamePaused false)
    (Variables|/Script/Engine.PlayerController|SetbShowMouseCursor _returnvalue true)
    (Input|SetInputModeUIOnly _returnvalue 0 "DoNotLock" false)))

(event Input|KeyboardEvents|Escape
  (params (Key :type Key%20Structure :default "None"))
  (bind _returnvalue (Game|GetPlayerController 0))
  (:Pressed
    (bind _returnvalue_2 (UserInterface|CreateWidget "/Game/Blueprints/PauseMenu.PauseMenu_C"))
    (UserInterface|Viewport|AddtoViewport _returnvalue_2 0)
    (Variables|/Script/Engine.PlayerController|SetbShowMouseCursor _returnvalue true)
    (Input|SetInputModeUIOnly _returnvalue 0 "DoNotLock" false)
    (Game|SetGamePaused true)))

(fn ConstructionScript)

(fn UiCtrlHP
  (Variables|/Game/UIs/UI_Screen.UI_Screen_C|SethpRatio (Variables|Default|GetuiScreen) (/ (Math|Conversions|ToFloat(Integer) (Variables|Default|Gethp)) (Math|Conversions|ToFloat(Integer) (Variables|Default|GetinitialHp))))
  (Variables|/Game/UIs/UI_Screen.UI_Screen_C|SethpString (Variables|Default|GetuiScreen) (Utilities|String|Append (Utilities|String|ToString(Integer) (Variables|Default|Gethp)) "/" (Utilities|String|ToString(Integer) (Variables|Default|GetinitialHp)))))

(fn UiCtrlSP
  (Variables|/Game/UIs/UI_Screen.UI_Screen_C|SetspRatio (Variables|Default|GetuiScreen) (/ (Variables|Default|Getstamina) (Variables|Default|GetinitialStamina))))

(fn UiCtrlMagazine
  (Variables|/Game/UIs/UI_Screen.UI_Screen_C|SetmgzString (Variables|Default|GetuiScreen) (Utilities|String|Append (Utilities|String|ToString(Integer) (Variables|Default|Getmagazine)) "/" (Utilities|String|ToString(Integer) (Variables|Default|GetinitMagazine)))))