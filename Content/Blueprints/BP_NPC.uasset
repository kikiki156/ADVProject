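; BP_NPC is a talkable NPC that steps through dialogue lines and then sends the player to MazeMap.
; Each Talk call increments TalkIndex and shows that Dialogue entry in a lazily created WB_Dialogue widget, playing the mesh animation once at index zero.
; When the index reaches the array length, a WB_LoadingScreen fade-out runs and the level opens after a short delay.
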(event EventBeginPlay)

(event Collision|EventActorBeginOverlap
  (params (OtherActor :type Actor%20Object%20Reference)))

(event EventTick
  (params (DeltaSeconds :type Float%20%28single-precision%29)))

(event EventTalk
  (Math|Integer|IncrementInt (Variables|Default|GetTalkIndex)
    (:%20%20
      (if (<= (Variables|Default|GetTalkIndex) (Utilities|Array|Length (Variables|Default|GetDialogue)))
        (Variables|Default|GetUI
          (:then
            _)
          (:else
            (bind _returnvalue (UserInterface|CreateWidget "/Game/Dialogue/WB_Dialogue.WB_Dialogue_C" (Game|GetPlayerController 0)))
            (bind _output_get (Variables|Default|SetUI _returnvalue))
            (UserInterface|Viewport|AddtoViewport _output_get 0)))
        (Rendering|Components|TextRender|SetText (Variables|/Game/Dialogue/WB_Dialogue.WB_Dialogue_C|GetTalkText (Variables|Default|GetUI)) (Utilities|Text|ToText(String) (Utilities|Array|Get(acopy) (Variables|Default|GetDialogue) (Variables|Default|GetTalkIndex))))
        (if (== (Variables|Default|GetTalkIndex) 0)
          (Audio|Components|Audio|Play (Variables|Default|GetMesh) false))
        (if (>= (Variables|Default|GetTalkIndex) (Utilities|Array|Length (Variables|Default|GetDialogue)))
          (bind _returnvalue_2 (UserInterface|CreateWidget "/Game/LevelTransition/WB_LoadingScreen.WB_LoadingScreen_C" (Game|GetPlayerController 0)))
          (bind _output_get_2 (Variables|Default|SetFadeOut _returnvalue_2))
          (UserInterface|Viewport|AddtoViewport _output_get_2 0)
          (Default|FadeOut (Variables|Default|GetFadeOut))
          (Utilities|FlowControl|Delay 2.0)
          (Game|OpenLevel(byName) "MazeMap"))))))

(fn ConstructionScript)